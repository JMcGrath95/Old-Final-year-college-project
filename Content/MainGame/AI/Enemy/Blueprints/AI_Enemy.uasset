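; AI controller for BP_Enemy that runs the BT_Enemy behavior tree and tracks whether the player is detected.
; On start it seeds the blackboard with patrol path settings and clears CanSeePlayer.
; Perception updates set CanSeePlayer from either of two index-matched senses, with only the first verifying the player's location.
; When the first sense fails and the player is distant, a delayed LostPlayer timer clears the flag unless re-detection cancels it.
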(event `self.ReceiveBeginPlay`
  ;[1 1 1] On start runs function to set up behaviour tree
  (`self.SetUpBehaviourTree`))

(event `self.AIPerception.OnPerceptionUpdated`
  (params (UpdatedActors :type "Array of Actor Object Reference (by ref)"))
  ;[1 1 1] on perception update it gets all the senses and passes them into function
  (for _array_element UpdatedActors
    (bind _info (`AIPerceptionComponent.GetActorsPerception` (`self.AIPerception`) _array_element))
    (`self.Set Up Senses` (`.LastSensedStimuli` (break `ActorPerceptionBlueprintInfo` _info)))))

(fn `LostPlayer`
  (`BlackboardComponent.SetValueAsBool` (`AIBlueprintHelperLibrary.GetBlackboard` null) "CanSeePlayer" false))

(fn `Set Up Senses`
  (params (AiSenses :type "Array of AIStimulus Structure"))
  (locals (CanSeePlayer :type Boolean))
  ;[1 1 1] Checks all types of perception if they detect player and updates blackboard
  (for (_array_element _array_index) AiSenses
    (switch `int` _array_index
      (:`0`
        (bind (_age _expirationage _strength _stimuluslocation _receiverlocation _tag _bsuccessfullysensed) (break `AIStimulus` _array_element))
        (if _bsuccessfullysensed
          (if (== _stimuluslocation (`self.K2_GetActorLocation` (`GameplayStatics.GetPlayerCharacter` 0)))
            (`BlackboardComponent.SetValueAsBool` (`AIBlueprintHelperLibrary.GetBlackboard` null) "CanSeePlayer" true)
            (`KismetSystemLibrary.K2_ClearTimer` null "LostPlayer"))
          (elif (< (`KismetMathLibrary.Vector_Distance` (`self.K2_GetActorLocation` (`GameplayStatics.GetPlayerCharacter` 0)) (`self.K2_GetActorLocation` (`self.K2_GetPawn`))) 3500.0)
            _
            (elif (`BlackboardComponent.GetValueAsBool` (`AIBlueprintHelperLibrary.GetBlackboard` null) "CanSeePlayer")
              (`KismetSystemLibrary.K2_SetTimer` null "LostPlayer" 5.0)))))
      (:`1`
        (if _bsuccessfullysensed
          (`BlackboardComponent.SetValueAsBool` (`AIBlueprintHelperLibrary.GetBlackboard` null) "CanSeePlayer" true)
          (`KismetSystemLibrary.K2_ClearTimer` null "LostPlayer"))))))

(fn `SetUpBehaviourTree`
  ;[1 1 1] Runs behaviour tree than sets starting values for the patrol path
  (`self.RunBehaviorTree` "/Game/MainGame/AI/Enemy/Behaviour/BT_Enemy.BT_Enemy")
  (bind _asbp_enemy (cast `/Game/MainGame/AI/Enemy/Blueprints/BP_Enemy` (`self.K2_GetPawn`)))
  (bind _patrolpath (`/Game/MainGame/AI/Enemy/Blueprints/BP_Enemy.PatrolPath` _asbp_enemy))
  (`BlackboardComponent.SetValueAsBool` (`AIBlueprintHelperLibrary.GetBlackboard` null) "PatrolPathLooping" (`/Game/MainGame/AI/Enemy/Blueprints/BP_PatrolPath.IsLooping` _patrolpath))
  (`BlackboardComponent.SetValueAsInt` (`AIBlueprintHelperLibrary.GetBlackboard` null) "PatrolPathDirection" 1)
  (`BlackboardComponent.SetValueAsFloat` (`AIBlueprintHelperLibrary.GetBlackboard` null) "WaitTime" (`/Game/MainGame/AI/Enemy/Blueprints/BP_PatrolPath.WaitTime` _patrolpath))
  (`BlackboardComponent.SetValueAsBool` (`AIBlueprintHelperLibrary.GetBlackboard` null) "CanSeePlayer" false))

(fn `UserConstructionScript`)