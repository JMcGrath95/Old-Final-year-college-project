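; BP_BoostMaxHealth is a consumable inventory pickup that permanently raises the player's maximum health.
; Interacting adds its item info to the main character's inventory and destroys the world actor, with a leftover debug print.
; Using the item increases the Health component's MaxHealth and adds the same amount of current health.
; Tick spins the root in yaw by DeltaSeconds plus a constant each frame, so the speed depends on frame rate.
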(event `/Game/MainGame/InventorySystem/InteractInterface.Interact`
  (`KismetSystemLibrary.PrintString` "Mr. Crabs")
  (bind _asbp_main_character (cast `/Game/MainGame/Character/BP_Main_Character` (`GameplayStatics.GetPlayerCharacter` 0)))
  (`/Game/MainGame/InventorySystem/UI/UMG_Inventory.AddToInventory` (`/Game/MainGame/Character/BP_Main_Character.Inventory` _asbp_main_character) (`self.ItemInfoStruct`))
  (`self.K2_DestroyActor`))

(event `/Game/MainGame/InventorySystem/InteractInterface.UseItem`
  (bind _asbp_main_character (cast `/Game/MainGame/Character/BP_Main_Character` (`GameplayStatics.GetPlayerCharacter` 0)))
  (bind _health (`/Game/MainGame/Character/BP_Main_Character.Health` _asbp_main_character))
  (set `HealthComponent.MaxHealth` (+ (`HealthComponent.MaxHealth` _health) 10) _health)
  (`HealthComponent.AddHealth` _health 10))

(event `self.ReceiveTick`
  (params (DeltaSeconds :type "Float (single-precision)"))
  (`SceneComponent.K2_AddLocalRotation` (`self.DefaultSceneRoot`) (`KismetMathLibrary.MakeRotator` 0.0 0.0 (+ DeltaSeconds 1.0)) false false))

(fn `UserConstructionScript`
  (`parent.UserConstructionScript`))