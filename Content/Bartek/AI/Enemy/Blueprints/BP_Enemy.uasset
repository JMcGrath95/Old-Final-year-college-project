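; Enemy character Blueprint for melee combat, driven by the AI_Enemy controller's blackboard, with a camera-facing health bar.
; Attack plays a random montage, using stronger special attacks once HitCount reaches three, and sphere-traces from a hand socket on DealDamage notifies to damage the player.
; Incoming damage is reported to AI perception and doubled when the enemy cannot see the player.
; Surviving hits play a reaction and heal the player by that damage.
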(event `/Game/Bartek/AI/Enemy/Blueprints/BP_AICombatInterface.Attack`
  (bind _socketlocation (`self.SocketLocation`))
  (bind _output (`|GetArrayItem` (`self.SpecialAttackAnimations`) (`KismetMathLibrary.RandomIntegerInRange` 0 (- (`KismetArrayLibrary.Array_Length` (`self.SpecialAttackAnimations`)) 1))))
  ;[1 1 1] Plays attack montage when interface is called
  (if (>= (`BlackboardComponent.GetValueAsInt` (`AIBlueprintHelperLibrary.GetBlackboard` (`AIBlueprintHelperLibrary.GetAIController` self)) "HitCount") 3)
    (set `self.Damage` 75.0)
    (bind _notifyname (`|PlayMontage` (`self.Mesh`) _output)
      (:`OnNotifyBegin`
        (if (== _notifyname "DealDamage")
          (`BlackboardComponent.SetValueAsInt` (`AIBlueprintHelperLibrary.GetBlackboard` (`AIBlueprintHelperLibrary.GetAIController` self)) "HitCount" 0)
          (if (`KismetStringLibrary.EqualEqual_StrStr` (`KismetSystemLibrary.GetDisplayName` _output) "Attack_Uppercut_Montage")
            (set `self.SocketLocation` (`SceneComponent.GetSocketLocation` (`self.Mesh`) "hand_l"))
            (else
              (set `self.SocketLocation` (`SceneComponent.GetSocketLocation` (`self.Mesh`) "hand_r") :!label _label)))
          (bind _outhit (`KismetSystemLibrary.SphereTraceSingle` :`Start` _socketlocation :`End` (+ _socketlocation (* (`KismetMathLibrary.GetForwardVector` (`self.K2_GetActorRotation`)) 50.0)) :`Radius` 30.0 :`TraceChannel` "TraceTypeQuery2" :`DrawDebugType` "ForDuration" :`DrawTime` 3.0))
          (if (== (`.HitActor` (`GameplayStatics.BreakHitResult` _outhit)) (`GameplayStatics.GetPlayerCharacter` 0))
            (if (`Actor.bCanBeDamaged` (`.HitActor` (`GameplayStatics.BreakHitResult` _outhit)))
              (`GameplayStatics.ApplyDamage` (`.HitActor` (`GameplayStatics.BreakHitResult` _outhit)) (`self.Damage`) null self))))))
    (else
      (set `self.Damage` 50.0)
      (bind _notifyname_2 (`|PlayMontage` (`self.Mesh`) (`|GetArrayItem` (`self.AttackAnimations`) (`KismetMathLibrary.RandomIntegerInRange` 0 (- (`KismetArrayLibrary.Array_Length` (`self.AttackAnimations`)) 1))))
        (:`OnNotifyBegin`
          (if (== _notifyname_2 "DealDamage")
            (goto _label)))))))

(event `self.ReceiveAnyDamage`
  (params (Damage :type "Float (single-precision)") (DamageType :type "DamageType Object Reference") (InstigatedBy :type "Controller Object Reference") (DamageCauser :type "Actor Object Reference"))
  ;[1 1 1] When Ai gets hit it loses health gives that much health to the player
  (`AISense_Damage.ReportDamageEvent` self (`GameplayStatics.GetPlayerCharacter` 0))
  (bind _newdamage (`self.IsSneakAttack` Damage))
  (`HealthComponent.SubtractHealth` (`self.Health`) _newdamage)
  (bind _result (`self.CheckIsDead`))
  (if (not _result)
    (`|PlayMontage` (`self.Mesh`) (`|GetArrayItem` (`self.HitAnimations`) (`KismetMathLibrary.RandomIntegerInRange` 0 (- (`KismetArrayLibrary.Array_Length` (`self.HitAnimations`)) 1))) 0.5
      (:`then`
        (bind _asbp_main_character (cast `/Game/Bartek/Character/BP_Main_Character` (`GameplayStatics.GetPlayerCharacter` 0)))
        (`HealthComponent.AddHealth` (`/Game/Bartek/Character/BP_Main_Character.Health` _asbp_main_character) _newdamage)))))

(event `self.ReceiveBeginPlay`
  ;[1 1 1] Setup healthbar ui
  (bind _asenemy_healthbar_ui (cast `/Game/Bartek/AI/Enemy/UI/EnemyHealthbar_UI` (`WidgetComponent.GetUserWidgetObject` (`self.Widget`))))
  (set `/Game/Bartek/AI/Enemy/UI/EnemyHealthbar_UI.Enemy` self _asenemy_healthbar_ui))

(event `self.ReceiveTick`
  (params (DeltaSeconds :type "Float (single-precision)"))
  (bind _widget (`self.Widget`))
  ;[1 1 1] Rotate healthbar to face player camera
  (`SceneComponent.K2_SetWorldRotation` _widget (`KismetMathLibrary.FindLookAtRotation` (`SceneComponent.K2_GetComponentLocation` _widget) (`self.K2_GetActorLocation` (`GameplayStatics.GetPlayerCameraManager` 0))) false false))

(fn `CheckIsDead`
  (returns (result :type Boolean))
  (bind _isdead (`HealthComponent.IsDead` (`self.Health`)))
  (bind _asai_enemy (cast `/Game/Bartek/AI/Enemy/Blueprints/AI_Enemy` (`AIBlueprintHelperLibrary.GetAIController` self)))
  (`BlackboardComponent.SetValueAsBool` (`AIBlueprintHelperLibrary.GetBlackboard` _asai_enemy) "Dead" _isdead)
  (if _isdead
    (`SceneComponent.SetVisibility` (`self.Widget`) false true)
    (return _isdead)))

(fn `DistanceCheck`
  (returns (DistanceFromCharacter :type "Float (double-precision)"))
  (return (`self.GetDistanceTo` (`GameplayStatics.GetPlayerCharacter` 0))))

(fn `IsSneakAttack`
  (params (CurrentDamage :type "Float (double-precision)"))
  (returns (NewDamage :type Integer))
  (bind _asai_enemy (cast `/Game/Bartek/AI/Enemy/Blueprints/AI_Enemy` (`AIBlueprintHelperLibrary.GetAIController` self)))
  (if (`BlackboardComponent.GetValueAsBool` (`AIBlueprintHelperLibrary.GetBlackboard` _asai_enemy) "CanSeePlayer")
    (return (`KismetMathLibrary.FTrunc` CurrentDamage))
    (else
      (return (`KismetMathLibrary.FTrunc` (* CurrentDamage 2.0))))))

(fn `SetSpeed`
  (params (Sprint :type Boolean))
  (bind _charactermovement (`self.CharacterMovement`))
  ;[1 1 1] If Sprint is true then player speed is faster ther wise he goes back to regular walk speed
  (if Sprint
    (set `CharacterMovementComponent.MaxWalkSpeed` (`self.ChaseSpeed`) _charactermovement)
    (else
      (set `CharacterMovementComponent.MaxWalkSpeed` (`self.PatrolWalkSpeed`) _charactermovement))))

(fn `UserConstructionScript`)