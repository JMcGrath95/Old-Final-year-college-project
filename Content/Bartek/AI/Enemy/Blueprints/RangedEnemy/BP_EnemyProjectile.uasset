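; BP_EnemyProjectile is a ranged enemy projectile that damages the player on contact.
; On actor overlap with the player character, it casts to BP_Main_Character, subtracts Damage directly from the Health's CurrentHealth and destroys itself; any other overlap just destroys it.
; Tick also destroys it once its distance from StartPosition reaches MaxRange.
; The graphs contain no movement logic and never set StartPosition.
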(event `self.ReceiveActorBeginOverlap`
  (params (OtherActor :type "Actor Object Reference"))
  (bind _returnvalue (`GameplayStatics.GetPlayerCharacter` 0))
  (if (== OtherActor _returnvalue)
    (bind _asbp_main_character (cast `/Game/Bartek/Character/BP_Main_Character` _returnvalue))
    (bind _health (`/Game/Bartek/Character/BP_Main_Character.Health` _asbp_main_character))
    (set `HealthComponent.CurrentHealth` (- (`HealthComponent.CurrentHealth` _health) (`self.Damage`)) _health)
    (`self.K2_DestroyActor`)
    (else
      (`self.K2_DestroyActor`))))

(event `self.ReceiveTick`
  (params (DeltaSeconds :type "Float (single-precision)"))
  (if (>= (`KismetMathLibrary.Vector_Distance` (`self.StartPosition`) (`self.K2_GetActorLocation` self)) (`self.MaxRange`))
    (`self.K2_DestroyActor`)))

(fn `UserConstructionScript`)